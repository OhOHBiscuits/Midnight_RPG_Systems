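; Inventory system Blueprint that currently serves as a test harness for adding items.
; Pressing 6 calls TryAddItem with one DA_Bread and prints the result.
; Server remove, move and transfer calls and item lookups are placed but unwired, and the inventory-updated event is empty.
; The BPI getters for inventory system, type and test storage are empty stubs.
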(event `Inventory has Upated`)

(event `Key|Six`
  (params (Key :type "Key Structure"))
  (:`Pressed`
    (`self.Add Item To Inventory`)))

(event `Add Item To Inventory`
  (bind _returnvalue (`self.TryAddItem` "/Game/Core/InventorySystem/ItemData/Comsumables/Food/DA_Bread.DA_Bread" 1))
  (`KismetSystemLibrary.PrintString` (`KismetStringLibrary.Conv_BoolToString` _returnvalue)))

(fn `BPI_Get Inventory System`
  (returns (`Inventory System` :type "/Game/Core/InventorySystem/AC_InventorySystem Object Reference"))
  (return null))

(fn `BPI_Get Inventory Type`
  (returns (`Inventory Type` :type "GameplayTag Structure"))
  (return))

(fn `BPI_Get STORAGE Inventory System_TEST FUNCTION`
  (returns (`Inventory System` :type "/Game/Core/InventorySystem/AC_InventorySystem Object Reference"))
  (return null))