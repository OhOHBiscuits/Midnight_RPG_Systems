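; Base weapon actor that can be interacted with for pickup and exposes itself, its mesh and its interaction type through interface getters.
; Interact runs parent logic and flags it picked up unless equipped, with equipped state set through an interface event.
; If not picked up at BeginPlay, a looping timer box-traces between two mesh sockets with debug drawing.
; Hits only print the component name; no damage is applied.
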(event `Damage Trace Start`
  (bind _returnvalue (`KismetSystemLibrary.K2_SetTimerDelegate` (delegate `Test`) 0.3 true))
  (set `self.Trace Timer` _returnvalue))

(event `self.ReceiveBeginPlay`
  (if (not (`self.Is Picked up`))
    (`self.Damage Trace Start`)))

(event `Test`
  (`self.Damage Trace`))

(event `InteractionSystemInterface.Interact`
  (params (Interactor :type "Actor Object Reference"))
  (if (not (`self.Is Equipped`))
    (`parent.Interact` Interactor)
    (set `self.Is Picked up` true)))

(event `/Game/Core/Weapons_and_Tools/Interface/BPI_Weapon_Interface.BPI_Set Is Equipped`
  (params (`Is Equipped` :type Boolean))
  (set `self.Is Equipped` `Is Equipped`))

(fn `BPI Bet Skeilital mesh`
  (returns (`Weapon Mesh` :type "SkeletalMeshComponent Object Reference"))
  (return null))

(fn `BPI Get hit Trace Sockets`
  (returns (NewParam :type "/Game/Core/Weapons_and_Tools/Main/BP_Main_Weapon Object Reference"))
  (return null))

(fn `BPI Get Weapon`
  (returns (Weapon :type "/Game/Core/Weapons_and_Tools/Main/BP_Main_Weapon Object Reference"))
  (return self))

(fn `BPI Get Weapon Static Mesh`
  (returns (`Weapon Mesh` :type "StaticMeshComponent Object Reference"))
  (bind _mesh (`self.Mesh`)
    (:`then`
      (return _mesh))
    (:`else`)))

(fn `BPI_Get  Input Inventory`
  (returns (Input_Inventory :type "InventoryComponent Object Reference"))
  (return null))

(fn `BPI_Get  OUTput Inventory`
  (returns (Output_Inventory :type "InventoryComponent Object Reference"))
  (return null))

(fn `BPI_Get Inventory System`
  (returns (`Inventory System` :type "/Game/Core/InventorySystem/AC_InventorySystem Object Reference"))
  (return null))

(fn `BPI_Get Inventory Type`
  (returns (`Inventory Type` :type "GameplayTag Structure"))
  (return))

(fn `BPI_Get Look at Actor`
  (returns (`Look At Actor` :type "Actor Object Reference"))
  (return null))

(fn `BPI_Get Player Charater`
  (returns (`Player Charater` :type "Actor Object Reference"))
  (return null))

(fn `BPI_Get Player Controllor`
  (returns (`Player Controllor` :type "PlayerController Object Reference"))
  (return null))

(fn `BPI_Get Player State`
  (returns (`Player State` :type "PlayerState Object Reference"))
  (return null))

(fn `BPI_Get STORAGE Inventory System_TEST FUNCTION`
  (returns (`Inventory System` :type "/Game/Core/InventorySystem/AC_InventorySystem Object Reference"))
  (return null))

(fn `BPI_Get_Fuel System`
  (returns (`Fuel System` :type "FuelComponent Object Reference"))
  (return null))

(fn `Damage Trace`
  (bind _mesh (`self.Mesh`))
  (if (and (`SceneComponent.DoesSocketExist` _mesh (`self.StartTrace`)) (`SceneComponent.DoesSocketExist` _mesh (`self.EndTrace`)))
    (bind (_outhit _returnvalue) (`KismetSystemLibrary.BoxTraceSingle` :`Start` (`SceneComponent.GetSocketLocation` (`self.Mesh`) (`self.StartTrace`)) :`End` (`SceneComponent.GetSocketLocation` (`self.Mesh`) (`self.EndTrace`)) :`HalfSize` (`KismetMathLibrary.Conv_DoubleToVector` (`self.Radius`)) :`TraceChannel` (`self.Trace Channel`) :`DrawDebugType` "ForDuration"))
    (if _returnvalue
      (bind _output_get (set `self.Out Hit` _outhit))
      (`KismetSystemLibrary.PrintString` (`KismetSystemLibrary.GetDisplayName` (`.HitComponent` (`GameplayStatics.BreakHitResult` _output_get))) true true (struct :`G` 0.66 :`B` 1.0 :`A` 1.0) 10.0))
    (else
      (`KismetSystemLibrary.PrintString` "Need to Create Damge Sockets on Mesh"))))

(fn `Get interaction Type`
  (returns (`Interacting Type` :type "GameplayTag Structure"))
  (return (`self.Interaction Type`)))

(fn `GetInteractionSystem`
  (returns (ReturnValue :type "InteractionSystemComponent Object Reference"))
  (return null))

(fn `GetInteractionTypeTag`
  (returns (ReturnValue :type "GameplayTag Structure"))
  (return (`self.Interaction Type`)))

(fn `UserConstructionScript`
  (`parent.UserConstructionScript`))