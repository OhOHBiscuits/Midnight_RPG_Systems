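; RPG player controller that sets up Enhanced Input for the local player, opens the player menu and handles interaction.
; Interact takes the pawn's look-at actor, sending pickups through ServerInteract and calling other interactions directly.
; Interface calls forward actor destruction and fuel burning to Server events, with burn starting on the look-at actor's FuelComponent.
; Most interface getters are empty stubs, and keys 1 and 5 are inventory debug tests.
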(event `self.ReceiveBeginPlay`
  (bind _returnvalue (pcsubsystem `EnhancedInputLocalPlayerSubsystem` self))
  (`self.Get Player`)
  (if (`KismetSystemLibrary.IsServer`)
    (if (not (`KismetSystemLibrary.IsDedicatedServer`))
      (if (`self.IsLocalController` self) :!label _label
        (`EnhancedInputSubsystemInterface.AddMappingContext` _returnvalue "/Game/Input/IMC_Default.IMC_Default" 0 (struct))
        (`EnhancedInputSubsystemInterface.AddMappingContext` _returnvalue "/Game/Input/IMC_MouseLook.IMC_MouseLook" 0 (struct))))
    (else
      (goto _label))))

(event `EnhancedInput|/Game/Input/Actions/IA_OpenPlayerMenu`
  (params (ActionValue :type Boolean) (ElapsedSeconds :type "Float (double-precision)") (TriggeredSeconds :type "Float (double-precision)") (InputAction :type "InputAction Object Reference" :default "/Game/Input/Actions/IA_OpenPlayerMenu.IA_OpenPlayerMenu"))
  (:`Started`
    (bind _newvar (`self.NewVar`)
      (:`then`
        (`Widget.RemoveFromParent` _newvar))
      (:`else`
        _))
    (bind _returnvalue (`|CreateWidget` "/Game/Core/InventorySystem/UI/UI_Player_Menu.UI_Player_Menu_C"))
    (bind _output_get (set `self.NewVar` _returnvalue))
    (`UserWidget.AddToViewport` _returnvalue 0)
    (`UserWidget.AddToViewport` _output_get 0)))

(event `Key|One`
  (params (Key :type "Key Structure"))
  (:`Pressed`
    (message `/Game/Core/InventorySystem/BPI_Inventory_Interface.BPI_Get Inventory System` (`GameplayStatics.GetPlayerState` 0))
    (for _array_element _
      (bind (_itemdata _quantity) (break `InventoryItem` _array_element))
      (`KismetSystemLibrary.PrintString` (`KismetTextLibrary.Conv_TextToString` (`|FormatText` "{item}  = {count}" (`|ConvertAsset` _itemdata) _quantity))))))

(event `CustomEvent`)

(event `/Game/Core/InteractionSystem/BPI_InteractionSystem.BPI_Destroy_Actor`
  (params (Actor :type "Actor Object Reference"))
  (`self.SERVER_Destory_Actor` Actor))

(event `SERVER_Destory_Actor`
  (params (`Actor to Destory` :type "Actor Object Reference"))
  (`self.K2_DestroyActor` `Actor to Destory`))

(event `Server Interact`
  (params (Target :type "Object Object Reference"))
  (message `InteractionInterface.Interact` Target self))

(event `EnhancedInput|/Game/Input/Actions/IA_Interact`
  (params (ActionValue :type Boolean) (ElapsedSeconds :type "Float (double-precision)") (TriggeredSeconds :type "Float (double-precision)") (InputAction :type "InputAction Object Reference" :default "/Game/Input/Actions/IA_Interact.IA_Interact"))
  (:`Started`
    ; Gets what Actor the player is looking at from interact Trace
    (bind _look_at_actor (message `/Game/Core/InteractionSystem/BPI_InteractionSystem.BPI_Get Look at Actor` (`GameplayStatics.GetPlayerPawn` 0)))
    (`/Engine/EditorBlueprintResources/StandardMacros.IsValid` _look_at_actor
      (:`Is Valid`
        (bind _returnvalue (message `InteractionInterface.GetInteractionTypeTag` _look_at_actor))
        (if (== _returnvalue (struct :`TagName` "Interaction.Type.Pickup"))
          (`self.Server Interact` _look_at_actor)
          (else
            (message `InteractionInterface.Interact` _look_at_actor self)))))))

(event `Key|Five`
  (params (Key :type "Key Structure"))
  (:`Pressed`
    (bind _returnvalue (`InventoryComponent.TryAddItem` (`InventoryHelpers.GetInventoryComponent` (`GameplayStatics.GetPlayerState` 0)) "/Game/Core/InventorySystem/ItemData/Comsumables/Food/Vegitable/DA_Cauliflower.DA_Cauliflower" 2))
    (`KismetSystemLibrary.PrintString` (`KismetStringLibrary.Conv_BoolToString` _returnvalue))))

(event `Server_Start_Burn`
  (`self.StartBurn`))

(event `/Game/Core/FuleSystems/Interface/BPI_FuelSystem_Interface.BPI_Start Burn`
  (`self.Server_Start_Burn`))

(event `/Game/Core/FuleSystems/Interface/BPI_FuelSystem_Interface.BPI_Stop_Burn`)

(fn `BPI_Get  Input Inventory`
  (returns (Input_Inventory :type "InventoryComponent Object Reference"))
  (return null))

(fn `BPI_Get  OUTput Inventory`
  (returns (Output_Inventory :type "InventoryComponent Object Reference"))
  (return null))

(fn `BPI_Get Inventory System`
  (returns (`Inventory System` :type "/Game/Core/InventorySystem/AC_InventorySystem Object Reference"))
  (return null))

(fn `BPI_Get Inventory Type`
  (returns (`Inventory Type` :type "GameplayTag Structure"))
  (return))

(fn `BPI_Get Look at Actor`
  (returns (`Look At Actor` :type "Actor Object Reference"))
  (bind _look_at_actor (message `/Game/Core/InteractionSystem/BPI_InteractionSystem.BPI_Get Look at Actor` (`GameplayStatics.GetPlayerPawn` 0)))
  (return _look_at_actor))

(fn `BPI_Get Player Charater`
  (returns (`Player Charater` :type "Actor Object Reference"))
  (return null))

(fn `BPI_Get Player Controllor`
  (returns (`Player Controllor` :type "PlayerController Object Reference"))
  (return self))

(fn `BPI_Get Player State`
  (returns (`Player State` :type "PlayerState Object Reference"))
  (return (`GameplayStatics.GetPlayerState` 0)))

(fn `BPI_Get STORAGE Inventory System_TEST FUNCTION`
  (returns (`Inventory System` :type "/Game/Core/InventorySystem/AC_InventorySystem Object Reference"))
  (return null))

(fn `BPI_Get_Fuel System`
  (returns (`Fuel System` :type "FuelComponent Object Reference"))
  (return null))

(fn `Get interaction Type`
  (returns (`Interacting Type` :type "GameplayTag Structure"))
  (return))

(fn `Get Look at actor`
  (returns (`Look At Actor` :type "Actor Object Reference"))
  (bind _look_at_actor (message `/Game/Core/InteractionSystem/BPI_InteractionSystem.BPI_Get Look at Actor` (`GameplayStatics.GetPlayerPawn` 0)))
  (return _look_at_actor))

(fn `Get Look at Actory`
  (returns (LookAtActor :type "Actor Object Reference"))
  (bind _output_get (set `self.Look at Actor` (`/Game/Core/Player/BP_RPG_Character.LookAtActor` (`self.As BP RPG Character`))))
  (return _output_get))

(fn `Get Player`
  (returns (Player :type "/Game/Core/Player/BP_RPG_Character Object Reference"))
  (bind _asbp_rpg_character (cast `/Game/Core/Player/BP_RPG_Character` (`GameplayStatics.GetPlayerCharacter` 0)))
  (bind _output_get (set `self.As BP RPG Character` _asbp_rpg_character))
  (return _output_get))

(fn `StartBurn`
  (bind _returnvalue (`self.GetComponentByClass` (`self.Get Look at actor`) "/Script/RPGSystem.FuelComponent"))
  (`/Engine/EditorBlueprintResources/StandardMacros.IsValid` _returnvalue
    (:`Is Valid`
      (`FuelComponent.StartBurn` _returnvalue))))

(fn `UserConstructionScript`)