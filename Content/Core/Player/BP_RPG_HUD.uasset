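; RPG HUD Blueprint that opens the player's inventory-style screens: fuel, workstation crafting, storage, or any supplied widget class.
; Each show event removes the current OpenedUI widget, creates the new one and adds it to the viewport, keeping one screen open at a time.
; Workstation screens receive station data and owner; storage receives the player controller's inventory component.
; BPI_Get HUD returns itself; the other interface getters are empty.
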(event `Show Fule UI`
  (bind _opened_ui (`self.Opened_UI`)
    (:`then`
      (`Widget.RemoveFromParent` _opened_ui))
    (:`else`
      _))
  (bind _returnvalue (`|CreateWidget` "/Game/Core/FuleSystems/UI/UI_Player_AND_Fule.UI_Player_AND_Fule_C"))
  (bind _output_get (set `self.Opened_UI` _returnvalue))
  (`UserWidget.AddToViewport` _output_get 0))

(event `/Game/Core/Player/Player_Interface/BPI_PlayerInterface.BPI_Show_UI`
  (params (UI :type "UserWidget Class Reference"))
  (bind _opened_ui (`self.Opened_UI`)
    (:`then`
      (`Widget.RemoveFromParent` _opened_ui))
    (:`else`
      _))
  (bind _returnvalue (`|CreateWidget` UI))
  (bind _output_get (set `self.Opened_UI` _returnvalue))
  (`UserWidget.AddToViewport` _output_get 0))

(event `/Game/Core/Player/Player_Interface/BPI_PlayerInterface.BPI Show Crafing UI`
  (params (`Work Station Data` :type "WorkstationDataAsset Object Reference") (WorkStatson :type "WorkstationActor Object Reference"))
  (bind _opened_ui (`self.Opened_UI`)
    (:`then`
      (`Widget.RemoveFromParent` _opened_ui))
    (:`else`
      _))
  (bind _returnvalue (`|CreateWidget` "/Game/Core/FuleSystems/UI/UI_Player_AND_WorkStation.UI_Player_AND_WorkStation_C" null `Work Station Data` WorkStatson))
  (bind _output_get (set `self.Opened_UI` _returnvalue))
  (`UserWidget.AddToViewport` _output_get 0))

(event `/Game/Core/Player/Player_Interface/BPI_PlayerInterface.BPI_Show_Player And Storage`
  (bind _opened_ui (`self.Opened_UI`)
    (:`then`
      (`Widget.RemoveFromParent` _opened_ui))
    (:`else`
      _))
  (bind _returnvalue (`|CreateWidget` "/Game/Core/InventorySystem/UI/UI_Player_AND_Storage.UI_Player_AND_Storage_C" null (`InventoryHelpers.GetInventoryComponentFromObject` (`GameplayStatics.GetPlayerController` 0))))
  (bind _output_get (set `self.Opened_UI` _returnvalue))
  (`UserWidget.AddToViewport` _output_get 0))

(event `/Game/Core/Player/Player_Interface/BPI_PlayerInterface.BPI ShowFule Crafing UI`
  (params (`Work Station Data` :type "WorkstationDataAsset Object Reference") (WorkStatson :type "WorkstationActor Object Reference"))
  (bind _opened_ui (`self.Opened_UI`)
    (:`then`
      (`Widget.RemoveFromParent` _opened_ui))
    (:`else`
      _))
  (bind _returnvalue (`|CreateWidget` "/Game/Core/FuleSystems/UI/UI_Player_AND_Fule.UI_Player_AND_Fule_C"))
  (bind _output_get (set `self.Opened_UI` _returnvalue))
  (`UserWidget.AddToViewport` _output_get 0))

(fn `BPI_Get Charater Mesh`
  (returns (`Player Combat Mesh Mesh` :type "SkeletalMeshComponent Object Reference"))
  (return null))

(fn `BPI_Get HUD`
  (returns (Hud :type "HUD Object Reference"))
  (return self))

(fn `BPI_Get Movement Controlloer`
  (returns (`Movement System` :type "MovementComponent Object Reference"))
  (return null))

(fn `UserConstructionScript`)