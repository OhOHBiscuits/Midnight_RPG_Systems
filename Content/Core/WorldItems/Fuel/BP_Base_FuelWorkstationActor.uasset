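; Base world-item actor for fuel-burning workstations, which opens its world item UI when interacted with.
; A fuel component drives a Niagara effect that starts hidden, shows while burning and hides when the burn stops or fuel runs out.
; Interface getters expose the fuel component, with the fuel inventory as input and the byproduct inventory as output.
; Player-related getters are empty, and the burn-progress handler only splits remaining seconds into time units without using them.
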(event `self.ReceiveBeginPlay`
  (`SceneComponent.SetVisibility` (`self.Niagara`) false false))

(event `InteractionInterface.Interact`
  (params (Interactor :type "Actor Object Reference"))
  (`self.TriggerWorldItemUI` Interactor))

(event `self.FuelComponent.OnBurnStarted`
  (`SceneComponent.SetVisibility` (`self.Niagara`) true false))

(event `self.FuelComponent.OnFuelBurnProgress`
  (params (RemainingSeconds :type "Float (single-precision)"))
  (bind (_days _hours _minutes _seconds) (`KismetMathLibrary.BreakTimespan` (`KismetMathLibrary.FromSeconds` RemainingSeconds)))
  (set `self.Days` _days)
  (set `self.Hours` _hours)
  (set `self.Minutes` _minutes)
  (set `self.Seconds` _seconds))

(event `self.FuelComponent.OnBurnStopped`
  (`SceneComponent.SetVisibility` (`self.Niagara`) false false :!label _label))

(event `self.FuelComponent.OnFuelDepleted`
  (goto _label))

(fn `BPI_Get  Input Inventory`
  (returns (Input_Inventory :type "InventoryComponent Object Reference"))
  (return (`self.FuelInventory`)))

(fn `BPI_Get  OUTput Inventory`
  (returns (Output_Inventory :type "InventoryComponent Object Reference"))
  (return (`self.ByproductInventory`)))

(fn `BPI_Get Look at Actor`
  (returns (`Look At Actor` :type "Actor Object Reference"))
  (return null))

(fn `BPI_Get Player Charater`
  (returns (`Player Charater` :type "Actor Object Reference"))
  (return null))

(fn `BPI_Get Player Controllor`
  (returns (`Player Controllor` :type "PlayerController Object Reference"))
  (return null))

(fn `BPI_Get Player State`
  (returns (`Player State` :type "PlayerState Object Reference"))
  (return null))

(fn `BPI_Get_Fuel System`
  (returns (`Fuel System` :type "FuelComponent Object Reference"))
  (return (`self.FuelComponent`)))

(fn `GetInteractionTypeTag`
  (returns (ReturnValue :type "GameplayTag Structure"))
  (return (`self.InteractionTypeTag`)))

(fn `UserConstructionScript`
  (`SceneComponent.SetVisibility` (`self.Niagara`) false false))