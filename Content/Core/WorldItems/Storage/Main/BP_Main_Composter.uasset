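; Composter storage world item with an inventory component, exposing interaction and inventory interface functions.
; On BeginPlay it calls ServerAddItems, which waits briefly and then seeds the inventory with green apples and pineapples.
; GetInteractionType returns its interaction type variable, while the Interact event and the inventory interface getters are empty stubs.
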(event `Server Add Items`
  (params (NewParam :type Boolean))
  (`KismetSystemLibrary.Delay` 5.0)
  (`InventoryComponent.TryAddItem` (`self.InventoryComp`) "/Game/Core/InventorySystem/ItemData/Comsumables/Food/Fruit/DA_GreenApple.DA_GreenApple" 2)
  (`InventoryComponent.TryAddItem` (`self.InventoryComp`) "/Game/Core/InventorySystem/ItemData/Comsumables/Food/Fruit/DA_PineApple.DA_PineApple" 2))

(event `self.ReceiveBeginPlay`
  (`self.Server Add Items` false))

(event `InteractionInterface.Interact`
  (params (Interactor :type "Actor Object Reference")))

(fn `BPI_Get Inventory System`
  (returns (`Inventory System` :type "/Game/Core/InventorySystem/AC_InventorySystem Object Reference"))
  (return null))

(fn `BPI_Get Inventory Type`
  (returns (`Inventory Type` :type "GameplayTag Structure"))
  (return))

(fn `BPI_Get STORAGE Inventory System_TEST FUNCTION`
  (returns (`Inventory System` :type "/Game/Core/InventorySystem/AC_InventorySystem Object Reference"))
  (return null))

(fn `Get interaction Type`
  (returns (`Interacting Type` :type "GameplayTag Structure"))
  (return (`self.Interagtion Type`)))

(fn `UserConstructionScript`)