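; BP_StorageBase is a base actor for world storage items that players can interact with.
; Its construction script sets the static mesh from the WorldMesh of its item data when that data is valid.
; On Interact, it gets the HUD message interface from the interactor and tells it to show the player-and-storage message.
; The inventory, player, fuel and interaction interface getters are empty stubs.
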(event `InteractionSystemInterface.Interact`
  (params (Interactor :type "Actor Object Reference"))
  (bind _hud (message `/Game/Core/Player/Player_Interface/BPI_PlayerInterface.BPI_Get HUD` Interactor))
  (message `/Game/Core/Player/Player_Interface/BPI_PlayerInterface.BPI_Show_Player And Storage` _hud))

(fn `BPI_Get  Input Inventory`
  (returns (Input_Inventory :type "InventoryComponent Object Reference"))
  (return null))

(fn `BPI_Get  OUTput Inventory`
  (returns (Output_Inventory :type "InventoryComponent Object Reference"))
  (return null))

(fn `BPI_Get Look at Actor`
  (returns (`Look At Actor` :type "Actor Object Reference"))
  (return null))

(fn `BPI_Get Player Charater`
  (returns (`Player Charater` :type "Actor Object Reference"))
  (return null))

(fn `BPI_Get Player Controllor`
  (returns (`Player Controllor` :type "PlayerController Object Reference"))
  (return null))

(fn `BPI_Get Player State`
  (returns (`Player State` :type "PlayerState Object Reference"))
  (return null))

(fn `BPI_Get_Fuel System`
  (returns (`Fuel System` :type "FuelComponent Object Reference"))
  (return null))

(fn `GetInteractionSystem`
  (returns (ReturnValue :type "InteractionSystemComponent Object Reference"))
  (return null))

(fn `UserConstructionScript`
  (bind _itemdata_0 (`self.ItemData_0`)
    (:`then`
      (`StaticMeshComponent.SetStaticMesh` (`self.StaticMesh`) (`|ConvertAsset` (`ItemDataAsset.WorldMesh` _itemdata_0))))
    (:`else`)))