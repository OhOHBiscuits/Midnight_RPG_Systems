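; GA_Pickup is a Gameplay Ability that lets the player interact with the looked-at actor, as a pickup, when the inventory has room.
; On activation it commits, then checks the avatar's inventory component for free space.
; If there is room, Blueprint interface messages fetch the player character and its look-at actor, which receives an Interact message with that character.
; The ability ends immediately on either branch, leaving the pickup logic to the target.
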(event `self.K2_ActivateAbility`
  (bind _returnvalue (`self.GetAvatarActorFromActorInfo`))
  (`self.K2_CommitAbility`)
  (if (not (`InventoryComponent.IsInventoryFull` (`InventoryHelpers.GetInventoryComponent` _returnvalue)))
    (bind _player_charater (message `/Game/Core/InteractionSystem/BPI_InteractionSystem.BPI_Get Player Charater` _returnvalue))
    (bind _look_at_actor (message `/Game/Core/InteractionSystem/BPI_InteractionSystem.BPI_Get Look at Actor` _player_charater))
    (message `InteractionInterface.Interact` _look_at_actor _player_charater)
    (`self.K2_EndAbility`)
    (else
      (`self.K2_EndAbility`))))